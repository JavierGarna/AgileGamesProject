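; BP_FarmPlot is a farm plot actor that holds a single crop at a time.
; Plant spawns a BP_Crop at the plot's transform if the plot is empty, stores it as CurrentPlant and sets the plot as its owner.
; ClearPlot resets the planted flag and drops the crop reference without destroying the crop actor.
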(event `/Game/Blueprints/PlantInterface.Plant`
  (if (not (`self.IsPlanted`))
    (set `self.IsPlanted` true)
    (bind _returnvalue (`|SpawnActorFromClass` "/Game/Blueprints/BP_Crop.BP_Crop_C" (`self.GetTransform`) "Undefined" "MultiplyWithRoot" null true null))
    (set `self.CurrentPlant` _returnvalue)
    (`self.SetOwner` _returnvalue self)))

(event `/Game/Blueprints/ClearPlotInterface.ClearPlot`
  (set `self.IsPlanted` false)
  (set `self.CurrentPlant` null))

(fn `UserConstructionScript`)