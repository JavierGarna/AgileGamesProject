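; BP_EnemySpawner is an enemy spawner actor that creates a random enemy at its own transform on every Tick.
; Its SpawnEnemy event picks a class from EnemyClasses, always spawns despite collisions and passes in a starting Health.
; Tick also sets EnemyAmount to a constant negative one rather than counting down.
; Unconnected leftover nodes include a check that opens Village with the day game mode when EnemyAmount runs out.
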(event `self.ReceiveBeginPlay`)

(event `self.ReceiveTick`
  (params (DeltaSeconds :type "Float (single-precision)"))
  (`self.SpawnEnemy`)
  (set `self.EnemyAmount` (- 0 1)))

(event `SpawnEnemy`
  (bind _enemyclasses (`self.EnemyClasses`))
  (`|SpawnActorFromClass` (`|GetArrayItem` _enemyclasses (`KismetMathLibrary.RandomInteger` (+ (`KismetArrayLibrary.Array_LastIndex` _enemyclasses) 1))) (`self.GetTransform` self) "AlwaysSpawn" "MultiplyWithRoot" null 100.0 100.0 null))

(fn `UserConstructionScript`)