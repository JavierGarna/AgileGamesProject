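; Enemy character that chases the player, leaps at them when in range, and deals damage on contact.
; Tick updates an in-range flag, and each PawnSensing sighting either launches the enemy toward the player or starts an AI MoveTo, both only when not falling.
; An attack collision overlap damages the third-person character with a one-second cooldown, and incoming damage reduces health until the enemy is destroyed.
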(event `self.ReceiveTick`
  (params (DeltaSeconds :type "Float (single-precision)"))
  ;[0.05098 0.05098 0.05098] OnTick Event
  (if (<= (`KismetMathLibrary.VSize` (- (`self.K2_GetActorLocation` (`GameplayStatics.GetPlayerCharacter` 0)) (`self.K2_GetActorLocation`))) (`self.AttackRange`))
    (set `self.canAttack` true)
    (else
      (set `self.canAttack` false))))

(event `self.PawnSensing.OnSeePawn`
  (params (Pawn :type "Pawn Object Reference"))
  ;[0.05098 0.05098 0.05098] OnSeePawn Event
  (set `self.IsSeeingPlayer` true)
  (if (`self.canAttack`)
    (`self.LaunchEnemy`)
    (elif (not (`NavMovementComponent.IsFalling` (`self.CharacterMovement`)))
      (`self.FollowPlayer`))))

(event `FollowPlayer`
  ;[0.05098 0.05098 0.05098] FollowPlayer Event
  (if (`self.IsSeeingPlayer`)
    (`|AIMoveTo` self (0.0 0.0 0.0) (`GameplayStatics.GetPlayerCharacter` 0))))

(event `self.ReceiveAnyDamage`
  (params (Damage :type "Float (single-precision)") (DamageType :type "DamageType Object Reference") (InstigatedBy :type "Controller Object Reference") (DamageCauser :type "Actor Object Reference"))
  ;[0.05098 0.05098 0.05098] AnyDamage Event
  (bind _output_get (set `self.Health` (- (`self.Health`) Damage)))
  (if (<= _output_get 0.0)
    (`self.K2_DestroyActor`)))

(event `LaunchEnemy`
  (bind (_returnvalue_x _returnvalue_y) (`KismetMathLibrary.BreakVector` (* (`KismetMathLibrary.Normal` (- (`self.K2_GetActorLocation` (`GameplayStatics.GetPlayerCharacter` 0)) (`self.K2_GetActorLocation`))) (`self.LaunchForce`))))
  ;[0.05098 0.05098 0.05098] LaunchEnemy Event
  (if (not (`NavMovementComponent.IsFalling` (`self.CharacterMovement`)))
    (`self.LaunchCharacter` (`KismetMathLibrary.MakeVector` _returnvalue_x _returnvalue_y 500.0) true true)))

(event `self.Attack Collision.OnComponentBeginOverlap`
  (params (OverlappedComponent :type "PrimitiveComponent Object Reference") (OtherActor :type "Actor Object Reference") (OtherComp :type "PrimitiveComponent Object Reference") (OtherBodyIndex :type Integer) (bFromSweep :type Boolean) (SweepResult :type "HitResult Structure (by ref)"))
  ;[0.05098 0.05098 0.05098] OnPlayerHit Event
  (bind _asbp_third_person_character (cast `/Game/ThirdPerson/Blueprints/BP_ThirdPersonCharacter` OtherActor))
  (if (`self.CanDealDamage`)
    (set `self.CanDealDamage` false)
    (`GameplayStatics.ApplyDamage` _asbp_third_person_character (`self.DamageAmount`) null self)
    (`KismetSystemLibrary.Delay` 1.0)
    (set `self.CanDealDamage` true)))

(fn `UserConstructionScript`)