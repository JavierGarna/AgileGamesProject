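; Enemy spawner actor that runs numbered waves, each sized by wave number times EnemiesPerWave.
; StartWave spawns EnemyClass at random Locatons entries and tracks the actors in AvctiveEnemies.
; Its Delay sits inside a plain for loop, which does not wait, so spawns are not staggered per enemy.
; After WaveInterval it calls the empty OnEnemyDefeat if the array is empty; nothing here removes enemies or calls StartWave.
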(event `StartWave`
  (bind _result (`/Engine/EditorBlueprintResources/StandardMacros.IncrementInt` (`self.WaveNumer`))
    (:`  `
      (bind _output_get (set `self.WaveNumer` _result))
      (for _ (range (* _output_get (`self.EnemiesPerWave`)))
        (`KismetSystemLibrary.Delay` (`self.SpawnInterval`))
        (bind _returnvalue (`|SpawnActorFromClass` (`self.EnemyClass`) (`KismetMathLibrary.MakeTransform` (`KismetArrayLibrary.Array_Random` (`self.Locatons`))) "AdjustIfPossibleButDontSpawnIfColliding" "MultiplyWithRoot" null 100.0 100.0 null))
        (`KismetArrayLibrary.Array_Add` (`self.AvctiveEnemies`) _returnvalue))
      (`KismetSystemLibrary.Delay` (`self.WaveInterval`))
      (if (`KismetArrayLibrary.Array_IsEmpty` (`self.AvctiveEnemies`))
        (`self.OnEnemyDefeat`)))))

(event `OnEnemyDefeat`)

(fn `UserConstructionScript`)