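; BP_FarmingArea is a zone actor that makes farming controls available only while the player is inside it.
; When a BP_ThirdPersonCharacter controlled by a BP_PlayerController begins overlapping its Boundary component, it adds the IMC_Farming Enhanced Input mapping context to that player's subsystem.
; End overlap removes the context, and both changes are written to the log.
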(event `self.Boundary.OnComponentBeginOverlap`
  (params (OverlappedComponent :type "PrimitiveComponent Object Reference") (OtherActor :type "Actor Object Reference") (OtherComp :type "PrimitiveComponent Object Reference") (OtherBodyIndex :type Integer) (bFromSweep :type Boolean) (SweepResult :type "HitResult Structure (by ref)"))
  ;[1 1 1] Add Farming input mapping
  (bind _asbp_third_person_character (cast `/Game/ThirdPerson/Blueprints/BP_ThirdPersonCharacter` OtherActor))
  (bind _asbp_player_controller (cast `/Game/Blueprints/BP_PlayerController` (`Pawn.GetController` _asbp_third_person_character)))
  (bind _returnvalue (pcsubsystem `EnhancedInputLocalPlayerSubsystem` _asbp_player_controller))
  (`/Engine/EditorBlueprintResources/StandardMacros.IsValid` _returnvalue
    (:`Is Valid`
      (`EnhancedInputSubsystemInterface.AddMappingContext` _returnvalue "/Game/ThirdPerson/Input/IMC_Farming.IMC_Farming" 0 (struct))
      (`VisualLoggerKismetLibrary.LogText` null "mapping context added" "VisLogBP" true))))

(event `self.Boundary.OnComponentEndOverlap`
  (params (OverlappedComponent :type "PrimitiveComponent Object Reference") (OtherActor :type "Actor Object Reference") (OtherComp :type "PrimitiveComponent Object Reference") (OtherBodyIndex :type Integer))
  ;[1 1 1] Remove farming input mapping
  (bind _asbp_third_person_character (cast `/Game/ThirdPerson/Blueprints/BP_ThirdPersonCharacter` OtherActor))
  (bind _asbp_player_controller (cast `/Game/Blueprints/BP_PlayerController` (`Pawn.GetController` _asbp_third_person_character)))
  (bind _returnvalue (pcsubsystem `EnhancedInputLocalPlayerSubsystem` _asbp_player_controller))
  (`/Engine/EditorBlueprintResources/StandardMacros.IsValid` _returnvalue
    (:`Is Valid`
      (`EnhancedInputSubsystemInterface.RemoveMappingContext` _returnvalue "/Game/ThirdPerson/Input/IMC_Farming.IMC_Farming" (struct))
      (`VisualLoggerKismetLibrary.LogText` null "mapping context removed" "VisLogBP" true))))

(fn `UserConstructionScript`)