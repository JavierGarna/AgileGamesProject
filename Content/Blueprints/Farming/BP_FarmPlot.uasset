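; Farm plot actor that takes a planting, grows it on a timer and yields a BP_Crop.
; Plant ignores occupied plots, decrements the player character's seed counter and shows a temporary mesh component for GrowTime.
; It then swaps that mesh for a spawned BP_Crop owned by the plot and stored as CurrentPlant.
; ClearPlot frees the plot and increments the player's crop counter.
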(event `/Game/Blueprints/Farming/PlantInterface.Plant`
  (if (not (`self.IsPlanted`))
    (set `self.IsPlanted` true)
    (bind _asbp_third_person_character (cast `/Game/ThirdPerson/Blueprints/BP_ThirdPersonCharacter` (`GameplayStatics.GetPlayerCharacter` 0)))
    (message `/Game/Blueprints/Farming/DecreaseSeedsCounterInterface.DecreaseSeedsCounter` _asbp_third_person_character)
    (bind _returnvalue (`AddComponent|NODE_AddStaticMeshComponent-0` :`RelativeTransform` (`self.StaticMeshesTransform`)))
    (`KismetSystemLibrary.Delay` (`self.GrowTime`))
    (`ActorComponent.K2_DestroyComponent` _returnvalue)
    (bind _returnvalue_2 (`|SpawnActorFromClass` "/Game/Blueprints/Farming/BP_Crop.BP_Crop_C" (`self.GetTransform`) "Undefined" "MultiplyWithRoot" null true null))
    (set `self.CurrentPlant` _returnvalue_2)
    (`self.SetOwner` _returnvalue_2 self)))

(event `/Game/Blueprints/Farming/ClearPlotInterface.ClearPlot`
  (set `self.IsPlanted` false)
  (set `self.CurrentPlant` null)
  (bind _asbp_third_person_character (cast `/Game/ThirdPerson/Blueprints/BP_ThirdPersonCharacter` (`GameplayStatics.GetPlayerCharacter` 0)))
  (message `/Game/Blueprints/Farming/IncreaseCropsCounterInterface.IncreaseCropsCounter` _asbp_third_person_character))

(fn `UserConstructionScript`)